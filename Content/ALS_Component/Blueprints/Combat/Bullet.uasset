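; Bullet projectile that triggers enemy hit reactions and surface-specific impact effects.
; The first non-owner sphere overlap runs a sphere trace, whose end is the forward vector scaled without adding the start location.
; Enemy-tagged hits call HitReact on their ALS component.
; The hit's physical material selects a DT_Impact_VFX row for CheckImpact, which spawns sound, particles and a randomly sized decal, then destroys the bullet.
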(event `self.Sphere.OnComponentBeginOverlap`
  (params (OverlappedComponent :type "PrimitiveComponent Object Reference") (OtherActor :type "Actor Object Reference") (OtherComp :type "PrimitiveComponent Object Reference") (OtherBodyIndex :type Integer) (bFromSweep :type Boolean) (SweepResult :type "HitResult Structure (by ref)"))
  (bind (_returnvalue_location _returnvalue_rotation) (`KismetMathLibrary.BreakTransform` (`SceneComponent.K2_GetComponentToWorld` (`self.Sphere`))))
  (if (!= OtherActor (`self.GetOwner`))
    (`/Engine/EditorBlueprintResources/StandardMacros.DoOnce` false
      (:`Completed`
        (bind _outhit (`KismetSystemLibrary.SphereTraceSingle` _returnvalue_location (* (`KismetMathLibrary.GetForwardVector` _returnvalue_rotation) 100.0) 5.0 "TraceTypeQuery1" true (`|MakeArray` (`self.GetOwner`))))
        (bind (_bblockinghit _binitialoverlap _time _distance _location _impactpoint _normal _impactnormal _physmat _hitactor _hitcomponent _hitbonename) (`GameplayStatics.BreakHitResult` _outhit))
        (if _bblockinghit
          (if (`self.ActorHasTag` _hitactor "Enemy")
            (bind _als_comp (`/Game/ALS_Component/Blueprints/Libraries/ALS_FunctionLib.Get_ALS_Comp` _hitactor))
            (`/Engine/EditorBlueprintResources/StandardMacros.IsValid` _als_comp
              (:`Is Valid`
                (`/Game/ALS_Component/Blueprints/CharacterLogic/ALS_Component.HitReact` _als_comp _hitbonename _impactnormal))))
          (bind _returnvalue (`|GetDataTableRow` "/Game/ALS_Component/Data/DataTables/DT_Impact_VFX.DT_Impact_VFX" (`/Game/ALS_Component/Blueprints/Libraries/ALS_FunctionLib.Get_PhysicMaterialName` _physmat))
            (:`then`
              (`self.Check Impact` _returnvalue (`SphereComponent.SphereRadius` (`self.Sphere`)) _outhit))))))))

(fn `Check Impact`
  (params (WSettings :type "/Game/ALS_Component/Data/Structs/ST_Impact_VFX Structure") (ImRadius :type "Float (double-precision)") (Hit :type "HitResult Structure (by ref)"))
  (bind (_bblockinghit _binitialoverlap _time _distance _location _impactpoint _normal _impactnormal _physmat _hitactor _hitcomponent _hitbonename) (`GameplayStatics.BreakHitResult` Hit))
  (bind ((`Particle_30_94175F3447B4B626F29076A6DBEA5046` _particle) (`Niagara_41_374CA7DA4931C05A719EDD9F5D89C479` _niagara)) (break `/Game/ALS_Component/Data/Structs/ST_Impact_VFX` (`local.WSettings`)))
  (bind _returnvalue (`KismetMathLibrary.Conv_VectorToRotator` _impactnormal))
  ;[0 1 0.4049] Impact SFX, VFX, Decal
  (`GameplayStatics.SpawnSoundAttached` (`.Sound_23_D75B8AD2420D9889DC0F808EE60F56E5` (break `/Game/ALS_Component/Data/Structs/ST_Impact_VFX` WSettings)) _hitcomponent "None" _location (struct) "KeepRelativeOffset" true 1.0 1.0 0.0 null null)
  (`/Game/ALS_Component/Blueprints/Libraries/ALS_FunctionLib.VFX_Check_OnLocation` _particle _niagara (`KismetMathLibrary.MakeTransform` _location _returnvalue))
  (`GameplayStatics.SpawnDecalAttached` (`.Decal_26_DB3BE74A4AC58A5526A6C8A18833B64A` (break `/Game/ALS_Component/Data/Structs/ST_Impact_VFX` (`local.WSettings`))) (* (`KismetMathLibrary.Conv_DoubleToVector` (`local.ImRadius`)) (`KismetMathLibrary.RandomFloatInRange` 0.75 1.9)) _hitcomponent _hitbonename _location _returnvalue "KeepWorldPosition" 5.0)
  (`self.K2_DestroyActor`))

(fn `UserConstructionScript`)