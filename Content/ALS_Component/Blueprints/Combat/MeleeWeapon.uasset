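; Melee weapon Blueprint that detects hits on enemies and triggers their hit reactions through the ALS component.
; While Condition is true, Tick sphere-traces against Pawns between the Start and End components, ignoring the owner.
; An initial-overlap hit tagged Enemy on actor or component stores the surface type and passes any bone name and impact normal to HitReact.
; That hit then clears Condition, ending detection until it is set again.
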(event `self.ReceiveTick`
  (params (DeltaSeconds :type "Float (single-precision)"))
  (if (`self.Condition`)
    (bind _outhit (`KismetSystemLibrary.SphereTraceSingleForObjects` (`SceneComponent.K2_GetComponentLocation` (`self.start`)) (`SceneComponent.K2_GetComponentLocation` (`self.end`)) 10.0 (`|MakeArray` "ObjectTypeQuery3" :!type "EObjectTypeQuery Enum") false (`|MakeArray` (`self.GetOwner`)) "None" true (struct :`R` 1.0 :`A` 1.0) (struct :`G` 1.0 :`A` 1.0) 1.0))
    (bind (_bblockinghit _binitialoverlap _time _distance _location _impactpoint _normal _impactnormal _physmat _hitactor _hitcomponent _hitbonename) (`GameplayStatics.BreakHitResult` _outhit))
    (`/Engine/EditorBlueprintResources/StandardMacros.IsValid` _hitactor
      (:`Is Valid`
        (if (and (!= (`self.Hit Actor`) _hitactor) _binitialoverlap (or (`self.ActorHasTag` _hitactor "Enemy") (`ActorComponent.ComponentHasTag` _hitcomponent "Enemy")))
          (set `self.Hit Actor` _hitactor)
          (set `self.Surface` (`PhysicalMaterial.SurfaceType` _physmat))
          (if (not (== _hitbonename "None"))
            (`/Game/ALS_Component/Blueprints/CharacterLogic/Actor_Components/ALS_Component.HitReact` (`/Game/ALS_Component/Blueprints/Libraries/ALS_FunctionLib.Get_ALS_Comp` _hitactor) _hitbonename _impactnormal))
          (set `self.Hit Actor` null)
          (set `self.Condition` false)
          (`KismetSystemLibrary.PrintString` "Hit" true true (struct :`R` 1.0 :`B` 0.12231 :`A` 1.0) 1.0))))))

(fn `UserConstructionScript`)