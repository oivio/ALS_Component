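; DamageVolume is a box volume that applies repeated damage to overlapping actors that have an ADV_PlayerStats component.
; On begin overlap, a Gate and Delay loop sends BaseDamage through EventUpdateShield every DamageRate interval.
; End overlap calls the same event with Recived false and zero damage, but does not close the gate, so nothing in the graph explicitly stops the loop.
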(event `self.Box.OnComponentBeginOverlap`
  (params (OverlappedComponent :type "PrimitiveComponent Object Reference") (OtherActor :type "Actor Object Reference") (OtherComp :type "PrimitiveComponent Object Reference") (OtherBodyIndex :type Integer) (bFromSweep :type Boolean) (SweepResult :type "HitResult Structure (by ref)"))
  (bind _returnvalue (`self.GetComponentByClass` OtherActor "/Game/ALS_Component/Blueprints/CharacterLogic/Actor_Components/ADV_PlayerStats.ADV_PlayerStats_C"))
  (`/Engine/EditorBlueprintResources/StandardMacros.IsValid` OtherActor
    (:`Is Valid`
      (`/Engine/EditorBlueprintResources/StandardMacros.IsValid` _returnvalue
        (:`Is Valid`
          (`|ExecutionSequence`
            (:`then_0`
              (goto _label :!via `Open`))
            (:`then_1`
              (`/Engine/EditorBlueprintResources/StandardMacros.Gate` true :!label _label
                (:`Exit`
                  (`/Game/ALS_Component/Blueprints/CharacterLogic/Actor_Components/ADV_PlayerStats.Event Update Shield` _returnvalue true (`self.Base Damage`))
                  (`KismetSystemLibrary.Delay` (`self.Damage_Rate`))
                  (goto _label))))))))))

(event `self.Box.OnComponentEndOverlap`
  (params (OverlappedComponent :type "PrimitiveComponent Object Reference") (OtherActor :type "Actor Object Reference") (OtherComp :type "PrimitiveComponent Object Reference") (OtherBodyIndex :type Integer))
  (bind _returnvalue (`self.GetComponentByClass` OtherActor "/Game/ALS_Component/Blueprints/CharacterLogic/Actor_Components/ADV_PlayerStats.ADV_PlayerStats_C"))
  (`/Engine/EditorBlueprintResources/StandardMacros.IsValid` OtherActor
    (:`Is Valid`
      (`/Engine/EditorBlueprintResources/StandardMacros.IsValid` _returnvalue
        (:`Is Valid`
          (`/Game/ALS_Component/Blueprints/CharacterLogic/Actor_Components/ADV_PlayerStats.Event Update Shield` _returnvalue false 0.0))))))

(fn `UserConstructionScript`)