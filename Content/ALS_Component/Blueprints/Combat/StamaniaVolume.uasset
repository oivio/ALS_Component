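; StamaniaVolume is a trigger volume that controls stamina regeneration for actors that carry an ADV_PlayerStats component.
; On Box begin overlap, it calls EventRegStamania on that component with regeneration enabled, passing the volume's RegRate and RegAmount.
; On end overlap, it calls the same event with default arguments, presumably to stop the regeneration.
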(event `self.Box.OnComponentBeginOverlap`
  (params (OverlappedComponent :type "PrimitiveComponent Object Reference") (OtherActor :type "Actor Object Reference") (OtherComp :type "PrimitiveComponent Object Reference") (OtherBodyIndex :type Integer) (bFromSweep :type Boolean) (SweepResult :type "HitResult Structure (by ref)"))
  (bind _returnvalue (`self.GetComponentByClass` OtherActor "/Game/ALS_Component/Blueprints/CharacterLogic/Actor_Components/ADV_PlayerStats.ADV_PlayerStats_C"))
  (`/Engine/EditorBlueprintResources/StandardMacros.IsValid` OtherActor
    (:`Is Valid`
      (`/Engine/EditorBlueprintResources/StandardMacros.IsValid` _returnvalue
        (:`Is Valid`
          (`/Game/ALS_Component/Blueprints/CharacterLogic/Actor_Components/ADV_PlayerStats.Event RegStamania` _returnvalue 0.0 true (`self.Reg Rate`) (`self.Reg Amount`)))))))

(event `self.Box.OnComponentEndOverlap`
  (params (OverlappedComponent :type "PrimitiveComponent Object Reference") (OtherActor :type "Actor Object Reference") (OtherComp :type "PrimitiveComponent Object Reference") (OtherBodyIndex :type Integer))
  (bind _returnvalue (`self.GetComponentByClass` OtherActor "/Game/ALS_Component/Blueprints/CharacterLogic/Actor_Components/ADV_PlayerStats.ADV_PlayerStats_C"))
  (`/Engine/EditorBlueprintResources/StandardMacros.IsValid` OtherActor
    (:`Is Valid`
      (`/Engine/EditorBlueprintResources/StandardMacros.IsValid` _returnvalue
        (:`Is Valid`
          (`/Game/ALS_Component/Blueprints/CharacterLogic/Actor_Components/ADV_PlayerStats.Event RegStamania` _returnvalue 0.0 false 0.0 0.0))))))

(fn `UserConstructionScript`)