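; Door actor in the ALS_Component folder that swings open when an actor enters its trigger box and closes when one leaves.
; Box overlaps play or reverse DoorTimeline, whose Yaw track is meant to rotate DoorRoot toward OpenRadius and toggle Open on finish.
; Overlaps also switch the ActionState on the other actor's ADV_Camera component, if present, but the door moves without requiring that component.
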(event `self.Box.OnComponentBeginOverlap`
  (params (OverlappedComponent :type "PrimitiveComponent Object Reference") (OtherActor :type "Actor Object Reference") (OtherComp :type "PrimitiveComponent Object Reference") (OtherBodyIndex :type Integer) (bFromSweep :type Boolean) (SweepResult :type "HitResult Structure (by ref)"))
  (bind _returnvalue (`self.GetComponentByClass` OtherActor "/Game/ADV_Camera/ADV_Camera.ADV_Camera_C"))
  (`/Engine/EditorBlueprintResources/StandardMacros.IsValid` OtherActor
    (:`Is Valid`
      (`/Engine/EditorBlueprintResources/StandardMacros.IsValid` _returnvalue
        (:`Is Valid`
          (set `/Game/ADV_Camera/ADV_Camera.Action State` "NewEnumerator12" _returnvalue))
        (:`Is Not Valid`
          _))
      (`TimelineComponent.Play` (`self.DoorTimeline`)))))

(event `self.Box.OnComponentEndOverlap`
  (params (OverlappedComponent :type "PrimitiveComponent Object Reference") (OtherActor :type "Actor Object Reference") (OtherComp :type "PrimitiveComponent Object Reference") (OtherBodyIndex :type Integer))
  (bind _returnvalue (`self.GetComponentByClass` OtherActor "/Game/ADV_Camera/ADV_Camera.ADV_Camera_C"))
  (`/Engine/EditorBlueprintResources/StandardMacros.IsValid` _returnvalue
    (:`Is Valid`
      (set `/Game/ADV_Camera/ADV_Camera.Action State` "NewEnumerator11" _returnvalue))
    (:`Is Not Valid`
      _))
  (`TimelineComponent.Reverse` (`self.DoorTimeline`)))

(fn `UserConstructionScript`)