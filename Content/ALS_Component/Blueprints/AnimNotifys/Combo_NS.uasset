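; Anim notify state that marks the combo window within an animation for the owner's ALS component.
; On begin, it registers itself as the component's ComboNotify and turns on EnableComboPeriod, which it clears on end.
; Each tick during the window, it calls JumpSectionForCombo on the component, leaving the section-jump logic to that component.
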(fn `Received_NotifyBegin`
  (params (MeshComp :type "SkeletalMeshComponent Object Reference") (Animation :type "AnimSequenceBase Object Reference") (TotalDuration :type "Float (double-precision)"))
  (returns (ReturnValue :type Boolean))
  (bind _returnvalue (`ActorComponent.GetOwner` MeshComp))
  (bind _als_comp (`/Game/ALS_Component/Blueprints/Libraries/ALS_FunctionLib.Get_ALS_Comp` _returnvalue _returnvalue))
  (`/Engine/EditorBlueprintResources/StandardMacros.IsValid` MeshComp
    (:`Is Valid`
      (set `/Game/ALS_Component/Blueprints/CharacterLogic/ALS_Component.Combo_Notify` self _als_comp)
      (set `/Game/ALS_Component/Blueprints/CharacterLogic/ALS_Component.EnableComboPeriod` true _als_comp)
      (return true))))

(fn `Received_NotifyEnd`
  (params (MeshComp :type "SkeletalMeshComponent Object Reference") (Animation :type "AnimSequenceBase Object Reference"))
  (returns (ReturnValue :type Boolean))
  (bind _returnvalue (`ActorComponent.GetOwner` MeshComp))
  (`/Engine/EditorBlueprintResources/StandardMacros.IsValid` MeshComp
    (:`Is Valid`
      (bind _output_get (set `/Game/ALS_Component/Blueprints/CharacterLogic/ALS_Component.EnableComboPeriod` false (`/Game/ALS_Component/Blueprints/Libraries/ALS_FunctionLib.Get_ALS_Comp` _returnvalue _returnvalue)))
      (return _output_get))))

(fn `Received_NotifyTick`
  (params (MeshComp :type "SkeletalMeshComponent Object Reference") (Animation :type "AnimSequenceBase Object Reference") (FrameDeltaTime :type "Float (double-precision)"))
  (returns (ReturnValue :type Boolean))
  (bind _returnvalue (`ActorComponent.GetOwner` MeshComp))
  (bind _als_comp (`/Game/ALS_Component/Blueprints/Libraries/ALS_FunctionLib.Get_ALS_Comp` _returnvalue _returnvalue))
  (`/Engine/EditorBlueprintResources/StandardMacros.IsValid` MeshComp
    (:`Is Valid`
      (`/Engine/EditorBlueprintResources/StandardMacros.IsValid` _als_comp
        (:`Is Valid`
          (`/Game/ALS_Component/Blueprints/CharacterLogic/ALS_Component.JumpSectionForCombo` _als_comp)
          (return true))))))