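; Anim notify state that sets a movement action on the owner's ALS component for the duration of an animation window.
; Begin sends the configured MovementAction to the component through an interface message.
; End resets it to a fixed enum value only if the current action still matches, leaving any action set by something else intact.
; The notify's display name includes the selected action.
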(fn `GetNotifyName`
  (returns (ReturnValue :type String))
  (return (`KismetStringLibrary.Concat_StrStr` "Movement Action: " (`|GetEnumeratorNameAsString` (`self.MovementAction`)))))

(fn `Received_NotifyBegin`
  (params (MeshComp :type "SkeletalMeshComponent Object Reference") (Animation :type "AnimSequenceBase Object Reference") (TotalDuration :type "Float (double-precision)"))
  (returns (ReturnValue :type Boolean))
  (bind _returnvalue (`ActorComponent.GetOwner` MeshComp))
  (message `/Game/ALS_Component/Blueprints/Interfaces/ALS_Character_BPI.BPI_Set_MovementAction` (`/Game/ALS_Component/Blueprints/Libraries/ALS_FunctionLib.Get_ALS_Comp` _returnvalue _returnvalue) (`self.MovementAction`))
  (return false))

(fn `Received_NotifyEnd`
  (params (MeshComp :type "SkeletalMeshComponent Object Reference") (Animation :type "AnimSequenceBase Object Reference"))
  (returns (ReturnValue :type Boolean))
  (bind _returnvalue (`ActorComponent.GetOwner` MeshComp))
  (bind _als_comp (`/Game/ALS_Component/Blueprints/Libraries/ALS_FunctionLib.Get_ALS_Comp` _returnvalue _returnvalue))
  (bind (_pawnmovementmode _movementstate _prevmovementstate _movementaction) (message `/Game/ALS_Component/Blueprints/Interfaces/ALS_Character_BPI.BPI_Get_CurrentStates` _als_comp))
  (if (`|EnumEquality` _movementaction (`self.MovementAction`))
    (message `/Game/ALS_Component/Blueprints/Interfaces/ALS_Character_BPI.BPI_Set_MovementAction` _als_comp "NewEnumerator4")
    (return false)
    (else
      (return false))))