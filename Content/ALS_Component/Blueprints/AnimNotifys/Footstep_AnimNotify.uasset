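; Footstep anim notify for the ALS component that plays surface-specific sound and visual effects for the left or right foot.
; It traces from the foot socket on the ALS mesh along the socket's forward axis, sign-flipped per foot, and uses the hit's physical surface type as the row name in DT_Footstep_VFX.
; The row drives attached sound, Niagara, particle and randomly sized decal spawns.
; The Mask_FootstepSound curve attenuates volume unless overridden.
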(fn `LineTrace`
  (params (AnimInstance :type "AnimInstance Object Reference") (MeshComp :type "SceneComponent Object Reference") (InSocketName :type Name) (End :type "Float (double-precision)") (DrawDebugType :type "EDrawDebugTrace Enum" :default "None"))
  (locals (StartLocation :type "Vector Structure" :default (0.0 0.0 0.0)) (ImpactLocation :type "Transform Structure"))
  (bind _als_comp (`/Game/ALS_Component/Blueprints/Libraries/ALS_FunctionLib.Get_ALS_Comp` (`ActorComponent.GetOwner` (`local.MeshComp`))))
  (bind (_returnvalue_location _returnvalue_rotation) (`KismetMathLibrary.BreakTransform` (`SceneComponent.GetSocketTransform` (`/Game/ALS_Component/Blueprints/CharacterLogic/ALS_Component.ALS_Mesh` _als_comp) (`local.InSocketName`) "RTS_World")))
  (bind _output_get (set `local.StartLocation` _returnvalue_location))
  (bind _outhit (`KismetSystemLibrary.LineTraceSingle` _output_get (+ _output_get (* (`KismetMathLibrary.GetForwardVector` _returnvalue_rotation) (`local.End`))) "TraceTypeQuery1" true (`|MakeArray` (`/Game/ALS_Component/Blueprints/CharacterLogic/ALS_Component.ALS_PlayerCharacter` _als_comp) :!type "Actor Object Reference") (`local.DrawDebugType`)))
  (bind (_bblockinghit _binitialoverlap _time _distance _location _impactpoint _normal _impactnormal _physmat) (`GameplayStatics.BreakHitResult` _outhit))
  (if (and _bblockinghit (`KismetSystemLibrary.IsValid` _physmat))
    (set `local.ImpactLocation` (`KismetMathLibrary.MakeTransform` _location (`KismetMathLibrary.Conv_VectorToRotator` _impactnormal)))
    (bind _returnvalue (`|GetDataTableRow` "/Game/ALS_Component/Data/DataTables/DT_Footstep_VFX.DT_Footstep_VFX" (`KismetStringLibrary.Conv_StringToName` (`|GetEnumeratorNameAsString` (`PhysicalMaterial.SurfaceType` _physmat))))
      (:`then`
        (bind (_sounds _particle _niagara _decal _decalsize _decalduration) (break `/Game/ALS_Component/Data/Structs/ST_Footstep_VFX` _returnvalue))
        (`self.RunVFX` _sounds _particle _niagara _decal _decalsize _decalduration (`local.ImpactLocation`) (`local.MeshComp`) (`local.AnimInstance`))
        (return))
      (:`RowNotFound`
        (return)))
    (else
      (return))))

(fn `Received_Notify`
  (params (MeshComp :type "SkeletalMeshComponent Object Reference") (Animation :type "AnimSequenceBase Object Reference"))
  (returns (ReturnValue :type Boolean))
  (bind _returnvalue (`SkeletalMeshComponent.GetAnimInstance` MeshComp))
  (bind _meshcomp (`local.MeshComp`))
  (bind _draw_debug_type (`self.Draw Debug Type`))
  (`/Engine/EditorBlueprintResources/StandardMacros.IsValid` MeshComp
    (:`Is Valid`
      (`/Engine/EditorBlueprintResources/StandardMacros.IsValid` _returnvalue
        (:`Is Valid`
          (if (`self.LeftFoot`)
            (`self.LineTrace` _returnvalue _meshcomp "Foot_L" -50.0 _draw_debug_type)
            (else
              (`self.LineTrace` _returnvalue _meshcomp "Foot_R" 50.0 _draw_debug_type)))
          (return false))))))

(fn `RunVFX`
  (params (FT_Sound :type "SoundBase Object Reference (by ref)") (Particle :type "ParticleSystem Object Reference") (Niagara :type "NiagaraSystem Object Reference") (Decal :type "MaterialInterface Object Reference") (DecalSize :type "Vector Structure") (LifeSpan :type "Float (double-precision)") (Location :type "Transform Structure") (Mesh :type "SceneComponent Object Reference") (AnimInst :type "AnimInstance Object Reference"))
  (bind _returnvalue (`KismetMathLibrary.RandomFloatInRange` 1.0 2.0))
  (bind (_location_location _location_rotation _location_scale) (`KismetMathLibrary.BreakTransform` (`local.Location`)))
  (bind (_location_location_2 _location_rotation_2) (`KismetMathLibrary.BreakTransform` (`local.Location`)))
  (bind (_location_location_3 _location_rotation_3) (`KismetMathLibrary.BreakTransform` (`local.Location`)))
  (bind _volumemultiplier (`self.VolumeMultiplier`))
  (`|ExecutionSequence`
    (:`then_0`
      (bind _ft_sound (`local.FT_Sound`)
        (:`then`
          (`GameplayStatics.SpawnSoundAttached` _ft_sound (`local.Mesh`) "root" (0.0 0.0 0.0) (struct) "KeepRelativeOffset" true (select `bool` (`self.OverrideMaskCurve`) :`false` (* (- 1.0 (`AnimInstance.GetCurveValue` (`local.AnimInst`) "Mask_FootstepSound")) _volumemultiplier) :`true` _volumemultiplier) (`self.PitchMultiplier`) 0.0 null null))
        (:`else`)))
    (:`then_1`
      (bind _niagara (`local.Niagara`)
        (:`then`
          (`NiagaraFunctionLibrary.SpawnSystemAtLocation` _niagara _location_location _location_rotation _location_scale))
        (:`else`)))
    (:`then_2`
      (bind _particle (`local.Particle`)
        (:`then`
          (`GameplayStatics.SpawnEmitterAtLocation` _particle _location_location_3 _location_rotation_3))
        (:`else`)))
    (:`then_3`
      (bind _decal (`local.Decal`)
        (:`then`
          (`GameplayStatics.SpawnDecalAtLocation` _decal (* (* (`local.DecalSize`) _returnvalue) _returnvalue) _location_location_2 _location_rotation_2 (`local.LifeSpan`)))
        (:`else`)))))