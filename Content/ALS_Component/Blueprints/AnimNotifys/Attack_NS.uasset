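; Attack_NS is an animation notify state that toggles the melee weapon's Condition flag during a window of an animation, apparently an attack.
; On begin it gets the mesh owner's ALS component and sets its MeleeWeapon's Condition to true.
; On end it sets the same flag back to false.
; Both events act only when the mesh and melee weapon are valid.
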(fn `Received_NotifyBegin`
  (params (MeshComp :type "SkeletalMeshComponent Object Reference") (Animation :type "AnimSequenceBase Object Reference") (TotalDuration :type "Float (double-precision)"))
  (returns (ReturnValue :type Boolean))
  (bind _returnvalue (`ActorComponent.GetOwner` MeshComp))
  (bind _meleeweapon (`/Game/ALS_Component/Blueprints/CharacterLogic/ALS_Component.MeleeWeapon` (`/Game/ALS_Component/Blueprints/Libraries/ALS_FunctionLib.Get_ALS_Comp` _returnvalue _returnvalue)))
  (`/Engine/EditorBlueprintResources/StandardMacros.IsValid` MeshComp
    (:`Is Valid`
      (`/Engine/EditorBlueprintResources/StandardMacros.IsValid` _meleeweapon
        (:`Is Valid`
          (bind _output_get (set `/Game/ALS_Component/Blueprints/CharacterLogic/MeleeWeapon.Condition` true _meleeweapon))
          (return _output_get))))))

(fn `Received_NotifyEnd`
  (params (MeshComp :type "SkeletalMeshComponent Object Reference") (Animation :type "AnimSequenceBase Object Reference"))
  (returns (ReturnValue :type Boolean))
  (bind _returnvalue (`ActorComponent.GetOwner` MeshComp))
  (bind _meleeweapon (`/Game/ALS_Component/Blueprints/CharacterLogic/ALS_Component.MeleeWeapon` (`/Game/ALS_Component/Blueprints/Libraries/ALS_FunctionLib.Get_ALS_Comp` _returnvalue _returnvalue)))
  (`/Engine/EditorBlueprintResources/StandardMacros.IsValid` MeshComp
    (:`Is Valid`
      (`/Engine/EditorBlueprintResources/StandardMacros.IsValid` _meleeweapon
        (:`Is Valid`
          (bind _output_get (set `/Game/ALS_Component/Blueprints/CharacterLogic/MeleeWeapon.Condition` false _meleeweapon))
          (return _output_get))))))