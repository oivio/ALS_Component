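; MeleeWeapon is a melee weapon Blueprint that detects hits and triggers hit reactions on enemies through their ALS component.
; While Condition is true, Tick sphere-traces between its Start and End points on the Visibility channel, ignoring the owner and drawing debug shapes.
; An initial-overlap hit clears Condition and stores surface type and impact point.
; Actors or components tagged Enemy receive HitReaction, and debug strings report hits.
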(event `self.ReceiveTick`
  (params (DeltaSeconds :type "Float (single-precision)"))
  (if (`self.Condition`)
    (bind _outhit (`KismetSystemLibrary.SphereTraceSingle` (`SceneComponent.K2_GetComponentLocation` (`self.start`)) (`SceneComponent.K2_GetComponentLocation` (`self.end`)) 5.0 "TraceTypeQuery1" false (`|MakeArray` (`self.GetOwner`)) "ForDuration" true (struct :`R` 1.0 :`A` 1.0) (struct :`G` 1.0 :`A` 1.0) 0.1))
    (bind (_bblockinghit _binitialoverlap _time _distance _location _impactpoint _normal _impactnormal _physmat _hitactor _hitcomponent) (`GameplayStatics.BreakHitResult` _outhit))
    (if _binitialoverlap
      (set `self.Condition` false)
      (set `self.Surface` (`PhysicalMaterial.SurfaceType` _physmat))
      (set `self.ImpactLocation` _impactpoint)
      (if (or (`self.ActorHasTag` _hitactor "Enemy") (`ActorComponent.ComponentHasTag` _hitcomponent "Enemy"))
        (`KismetSystemLibrary.PrintString` "Hit Enemy" true true (struct :`G` 0.66 :`B` 1.0 :`A` 1.0) 0.01)
        (`/Game/ALS_Component/Blueprints/CharacterLogic/ALS_Component.HitReaction` (`/Game/ALS_Component/Blueprints/Libraries/ALS_FunctionLib.Get_ALS_Comp` _hitactor) (`self.ImpactLocation`) _impactnormal)
        (else
          (`KismetSystemLibrary.PrintString` "Hit" true true (struct :`R` 1.0 :`G` 0.041141 :`B` 0.031194 :`A` 1.0) 1.0))))))

(fn `UserConstructionScript`)